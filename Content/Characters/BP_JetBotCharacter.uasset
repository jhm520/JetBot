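; BP_JetBotCharacter is the player character Blueprint for JetBot, layered on a parent class that handles movement events and death.
; Tick points the MovementDirection component along RealVelocity before calling the parent Tick.
; Capsule hits and GrindCapsule overlap begin and end events are forwarded to handler functions.
; Die runs parent logic, then resets time on BP_JetBotGameMode; destruction calls OnDeath, which notifies that game mode of the player's death.
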(event `self.ReceiveBeginPlay`)

(event `self.ReceiveDestroyed`
  (`self.OnDeath`))

(event `OnDeath`
  (bind _asbp_jet_bot_game_mode (cast `/Game/GameMode/BP_JetBotGameMode` (`GameplayStatics.GetGameMode`)))
  (`/Game/GameMode/BP_JetBotGameMode.OnPlayerDeath` _asbp_jet_bot_game_mode self))

(event `self.ReceiveTick`
  (params (DeltaSeconds :type "Float (single-precision)"))
  (`SceneComponent.K2_SetWorldRotation` (`self.MovementDirection`) (`KismetMathLibrary.FindLookAtRotation` (`KismetMathLibrary.MakeVector` 0.0) (`self.RealVelocity`)) false false)
  (`parent.ReceiveTick` DeltaSeconds))

(event `self.CapsuleComponent.OnComponentHit`
  (params (HitComponent :type "PrimitiveComponent Object Reference") (OtherActor :type "Actor Object Reference") (OtherComp :type "PrimitiveComponent Object Reference") (NormalImpulse :type "Vector Structure") (Hit :type "HitResult Structure (by ref)"))
  (`self.OnCapsuleComponentHit` HitComponent OtherActor OtherComp NormalImpulse Hit))

(event `self.GrindCapsule.OnComponentBeginOverlap`
  (params (OverlappedComponent :type "PrimitiveComponent Object Reference") (OtherActor :type "Actor Object Reference") (OtherComp :type "PrimitiveComponent Object Reference") (OtherBodyIndex :type Integer) (bFromSweep :type Boolean) (SweepResult :type "HitResult Structure (by ref)"))
  (`self.OnGrindCapsuleBeginOverlap` OverlappedComponent OtherActor OtherComp OtherBodyIndex bFromSweep))

(event `self.GrindCapsule.OnComponentEndOverlap`
  (params (OverlappedComponent :type "PrimitiveComponent Object Reference") (OtherActor :type "Actor Object Reference") (OtherComp :type "PrimitiveComponent Object Reference") (OtherBodyIndex :type Integer))
  (`self.OnGrindCapsuleEndOverlap` OverlappedComponent OtherActor OtherComp OtherBodyIndex))

(event `self.Die`
  (params (CauseOfDeath :type "ECauseOfDeathEnum Enum" :default "None"))
  (`parent.Die` CauseOfDeath)
  (bind _asbp_jet_bot_game_mode (cast `/Game/GameMode/BP_JetBotGameMode` (`GameplayStatics.GetGameMode`)))
  (`/Game/GameMode/BP_JetBotGameMode.ResetTime` _asbp_jet_bot_game_mode))

(fn `UserConstructionScript`)