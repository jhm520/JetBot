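; BP_LevelSpawner is a level-building actor that spawns a world tile when play begins.
; BeginPlay destroys and clears any tracked tiles, then spawns one BP_WorldTile at its root transform and stores it in TileArray.
; A custom event adds the first obstacle class as a child actor at a given transform.
; The construction script prints NumTiles and calls SpawnTiles, which is empty because its static mesh grid loop is disconnected.
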(event `self.ReceiveBeginPlay`
  (`|ExecutionSequence`
    (:`then_0`
      (for _array_element (`self.TileArray`)
        (`self.K2_DestroyActor` _array_element))
      (`KismetArrayLibrary.Array_Clear` (`self.TileArray`)))
    (:`then_1`
      (bind _returnvalue (`|SpawnActorFromClass` "/Game/Actors/WorldTiles/BP_WorldTile.BP_WorldTile_C" (`SceneComponent.K2_GetComponentToWorld` (`self.DefaultSceneRoot`)) "Undefined" "OverrideRootScale" null null))
      (`KismetArrayLibrary.Array_Add` (`self.TileArray`) _returnvalue))))

(event `self.SpawnObstacleAtTransform`
  (params (SpawnTransform :type "Transform Structure"))
  (bind _returnvalue (`AddComponent|NODE_AddChildActorComponent-1` :`RelativeTransform` SpawnTransform))
  (`ChildActorComponent.SetChildActorClass` _returnvalue (`|GetArrayItem` (`self.ObstacleClasses`))))

(fn `SpawnTiles`)

(fn `UserConstructionScript`
  (locals (SpawnLocation :type "Vector Structure" :default (-5000.0 -5000.0 0.0)))
  (`KismetSystemLibrary.PrintString` (`KismetStringLibrary.Conv_IntToString` (`self.NumTiles`)))
  (`self.SpawnTiles`))