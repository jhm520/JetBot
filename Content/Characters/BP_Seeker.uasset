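; BP_Seeker is a character Blueprint for the Seeker, with a toggleable flashlight.
; Pressing the Flashlight input action calls the SetFlashlight event with the inverse of the current state.
; SetFlashlight stores the new state and shows or hides the SpotLight component to match.
; The BeginPlay, overlap and Tick events are disabled stubs, and the construction script only calls its parent.
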(event `InputAction|Flashlight`
  (params (Key :type "Key Structure"))
  (:`Pressed`
    (`self.SetFlashlight` (not (`self.bFlashlight`)))))

(event `SetFlashlight`
  (params (bFlashlight :type Boolean))
  (bind _output_get (set `self.bFlashlight` bFlashlight))
  (`SceneComponent.SetVisibility` (`self.SpotLight`) _output_get false))

(fn `UserConstructionScript`
  (`parent.UserConstructionScript`))