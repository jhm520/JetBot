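; Player controller for a hide-and-seek game that assigns the monster pawn to players whose controller ID is not 0.
; Shortly after BeginPlay it runs ChoosePlayerPawn, which acts only with authority.
; For those players it destroys the current pawn, then spawns and possesses a BP_Monster at the first PlayerStart found.
; Controller 0 keeps its existing pawn.
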(event `self.ReceiveBeginPlay`
  (`KismetSystemLibrary.Delay` 0.2)
  (`self.ChoosePlayerPawn`))

(fn `ChoosePlayerPawn`
  (locals (LocalPawn :type "Pawn Object Reference"))
  (`/Engine/EditorBlueprintResources/ActorMacros.Switch Has Authority`
    (:`Authority`
      (if (!= (`GameplayStatics.GetPlayerControllerID` self) 0)
        (`self.K2_DestroyActor` (`self.K2_GetPawn`))
        (`self.UnPossess`)
        (`|ExecutionSequence`
          (:`then_0`
            (bind _outactors (`GameplayStatics.GetAllActorsOfClass` "/Script/Engine.PlayerStart"))
            (if (> (`KismetArrayLibrary.Array_Length` _outactors) 0)
              (bind _returnvalue (`|SpawnActorFromClass` "/Game/Characters/BP_Monster.BP_Monster_C" (`self.GetTransform` (`|GetArrayItem` _outactors)) "Undefined" "OverrideRootScale" null null))
              (`self.Possess` _returnvalue))))))))

(fn `UserConstructionScript`)