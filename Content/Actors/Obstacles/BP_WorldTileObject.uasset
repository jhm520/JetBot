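; BP_WorldTileObject is an obstacle actor that ties its lifetime to its owner and reveals its mesh when a JetBot character approaches.
; On BeginPlay it calls OnSpawnedByTileMessage if a BP_WorldTile owns it, and binds to any valid owner's OnDestroyed to destroy itself alongside it.
; When the character overlaps BoundaryBox, it unhides ObjectMesh and its children, then disables the box's overlap events so the reveal happens once.
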(event `self.ReceiveBeginPlay`
  (bind _returnvalue (`self.GetOwner`))
  (`|ExecutionSequence`
    (:`then_0`
      (cast `/Game/Actors/WorldTiles/BP_WorldTile` (`self.GetOwner`))
      (message `/Game/Actors/Obstacles/WorldTileObjectInterface.OnSpawnedByTile` self))
    (:`then_1`
      (`/Engine/EditorBlueprintResources/StandardMacros.IsValid` _returnvalue
        (:`Is Valid`
          (add `self.OnDestroyed` _returnvalue (delegate `DestroyThisToo`)))))))

(event `DestroyThisToo` :!signature `self.OnDestroyed`
  (params (DestroyedActor :type "Actor Object Reference"))
  (`self.K2_DestroyActor`))

(event `self.BoundaryBox.OnComponentBeginOverlap`
  (params (OverlappedComponent :type "PrimitiveComponent Object Reference") (OtherActor :type "Actor Object Reference") (OtherComp :type "PrimitiveComponent Object Reference") (OtherBodyIndex :type Integer) (bFromSweep :type Boolean) (SweepResult :type "HitResult Structure (by ref)"))
  (cast `/Game/Characters/BP_JetBotCharacter` OtherActor)
  (`SceneComponent.SetHiddenInGame` (`self.ObjectMesh`) false true)
  (set `PrimitiveComponent.bGenerateOverlapEvents` false (`self.BoundaryBox`)))

(fn `UserConstructionScript`)