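; Game mode for JetBot that picks and possesses a VR or non-VR pawn at startup and manages an endless world-tile path.
; OnTileEntered calls SpawnTilePath, which capsule-checks ahead along X and chains random tiles onto the leading tile.
; Tick tests one tracked tile per frame, destroying it once the player is far enough away.
; Initial-tile spawning is disconnected, surrounding-tile spawning is uncalled here, and several helpers are stubs.
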(event `self.ReceiveBeginPlay`
  (bind _returnvalue (`GameplayStatics.GetPlayerController` 0))
  (`/Engine/EditorBlueprintResources/StandardMacros.IsValid` (`GameplayStatics.GetPlayerCharacter` 0)
    (:`Is Valid`
      (set `self.DefaultPawnClass` "/Game/Characters/BP_NonVRCharacter.BP_NonVRCharacter_C" :!label _label))
    (:`Is Not Valid`
      (if (`self.bPlayAsVR`)
        (switch `name` (`HeadMountedDisplayFunctionLibrary.GetHMDDeviceName`)
          (:`Default`
            (goto _label))
          (:`SteamVR`
            (set `self.DefaultPawnClass` "/Game/Characters/BP_VRCharacter.BP_VRCharacter_C")))
        (else
          (goto _label)))))
  (`/Engine/EditorBlueprintResources/StandardMacros.IsValid` _returnvalue
    (:`Is Valid`
      (bind _returnvalue_2 (`|SpawnActorFromClass` (`self.DefaultPawnClass`) (`KismetMathLibrary.MakeTransform` (0.0 0.0 0.0)) "Undefined" "OverrideRootScale" _returnvalue null))
      (`Controller.Possess` _returnvalue _returnvalue_2)
      (`KismetSystemLibrary.ExecuteConsoleCommand` "viewmode unlit")
      (`KismetSystemLibrary.ExecuteConsoleCommand` "stat fps"))))

(event `self.ReceiveTick`
  (params (DeltaSeconds :type "Float (single-precision)"))
  (`self.CheckTileIsFarAway`))

(event `CheckTileIsFarAway`
  (bind _worldtilearray (`self.WorldTileArray`))
  (`|ExecutionSequence`
    (:`then_0`
      (if (> (`self.CheckTileIndex`) (- (`KismetArrayLibrary.Array_Length` _worldtilearray) 1))
        (set `self.CheckTileIndex` 0)))
    (:`then_1`
      (bind _asbp_world_tile (cast `/Game/Actors/WorldTiles/BP_WorldTile` (`|GetArrayItem` _worldtilearray (`self.CheckTileIndex`))))
      (bind _bfaraway (`self.IsPlayerFarAwayFromTile` _asbp_world_tile))
      (if _bfaraway
        (`KismetArrayLibrary.Array_Remove` (`self.WorldTileArray`) (`self.CheckTileIndex`))
        (`self.K2_DestroyActor` _asbp_world_tile)))
    (:`then_2`
      (`/Engine/EditorBlueprintResources/StandardMacros.IncrementInt` (`self.CheckTileIndex`)))))

(event `CheckTileObjectIsFarAway`)

(fn `AdjustTileSpawnOrientation`
  (params (SpawnedWorldTile :type "/Game/Actors/WorldTiles/BP_WorldTile Object Reference") (LeadingTile :type "/Game/Actors/WorldTiles/BP_WorldTile Object Reference"))
  (locals (LocalSpawnedTile :type "/Game/Actors/WorldTiles/BP_WorldTile Object Reference") (LocalLeadingTIle :type "/Game/Actors/WorldTiles/BP_WorldTile Object Reference"))
  (set `local.LocalLeadingTIle` LeadingTile)
  (set `local.LocalSpawnedTile` SpawnedWorldTile))

(fn `GetRandomObstacleClass`
  (returns (ReturnValue :type "Object Class Reference"))
  (bind _tileobjecttypes (`self.TileObjectTypes`))
  (return (`|GetArrayItem` _tileobjecttypes (`KismetMathLibrary.RandomIntegerInRange` 0 (- (`KismetArrayLibrary.Array_Length` _tileobjecttypes) 1)))))

(fn `IsPlayerFarAwayFromTile`
  (params (InWorldTile :type "/Game/Actors/WorldTiles/BP_WorldTile Object Reference"))
  (returns (bFarAway :type Boolean))
  (bind _returnvalue (`GameplayStatics.GetPlayerCharacter` 0))
  (bind _boxextent_x (`KismetMathLibrary.BreakVector` (`BoxComponent.BoxExtent` (`/Game/Actors/WorldTiles/BP_WorldTile.TileBoundaryBox` InWorldTile))))
  (bind _returnvalue_2 (+ (* (`self.TilePathLength`) (* _boxextent_x 2.0)) (/ _boxextent_x 2.0)))
  (`/Engine/EditorBlueprintResources/StandardMacros.IsValid` _returnvalue
    (:`Is Valid`
      (return (> (`KismetMathLibrary.VSize` (- (`self.K2_GetActorLocation` _returnvalue) (`self.K2_GetActorLocation` InWorldTile))) (`KismetMathLibrary.VSize` (`KismetMathLibrary.MakeVector` _returnvalue_2 _returnvalue_2 _returnvalue_2)))))
    (:`Is Not Valid`
      (return false))))

(fn `IsPlayerFarAwayFromTileObject`
  (params (InTileObject :type "/Game/Actors/Obstacles/BP_WorldTileObject Object Reference"))
  (returns (IsFarAway :type Boolean))
  (bind _returnvalue (`GameplayStatics.GetPlayerCharacter` 0))
  (`/Engine/EditorBlueprintResources/StandardMacros.IsValid` _returnvalue
    (:`Is Valid`
      (return (> (`KismetMathLibrary.VSize` (- (`self.K2_GetActorLocation` InTileObject) (`self.K2_GetActorLocation` _returnvalue))) 5000.0)))
    (:`Is Not Valid`
      (return true))))

(fn `IsWorldTileOrientationValid`
  (params (InWorldTile :type "/Game/Actors/WorldTiles/BP_WorldTile Object Reference"))
  (returns (bValid :type Boolean)))

(fn `OnTileEntered`
  (params (InWorldTile :type "/Game/Actors/WorldTiles/BP_WorldTile Object Reference"))
  (locals (PreviousCenterTile :type "/Game/Actors/WorldTiles/BP_WorldTile Object Reference"))
  (`self.SpawnTilePath` InWorldTile))

(fn `SpawnSurroundingTiles`
  (params (InWorldTile :type "/Game/Actors/WorldTiles/BP_WorldTile Object Reference"))
  (locals (LocalWorldTile :type "/Game/Actors/WorldTiles/BP_WorldTile Object Reference") (TileSpawnTransform :type "Transform Structure"))
  (bind _spawnrotations (`self.SpawnRotations`))
  (bind _worldtiletypearray (`self.WorldTileTypeArray`))
  (bind _surroundingtiles (`/Game/Actors/WorldTiles/BP_WorldTile.SurroundingTiles` (`local.LocalWorldTile`)))
  (bind _output_get (set `local.LocalWorldTile` InWorldTile))
  (`/Engine/EditorBlueprintResources/StandardMacros.IsValid` _output_get
    (:`Is Valid`
      (bind _output_get_2 (set `self.SurroundingTilesLength` (`KismetArrayLibrary.Array_Length` _surroundingtiles)))
      (for _index (range _output_get_2)
        (bind _returnvalue (`SceneComponent.K2_GetComponentLocation` (`|GetArrayItem` _surroundingtiles _index)))
        (bind (_outactors _returnvalue_2) (`KismetSystemLibrary.CapsuleOverlapActors` _returnvalue 1000.0 5000.0 (`|MakeArray` "ObjectTypeQuery7" :!type "EObjectTypeQuery Enum")))
        (if (not _returnvalue_2)
          (bind _returnvalue_3 (`|SpawnActorFromClass` (`|GetArrayItem` _worldtiletypearray (`KismetMathLibrary.RandomIntegerInRange` 0 (- (`KismetArrayLibrary.Array_Length` _worldtiletypearray) 1))) (`KismetMathLibrary.MakeTransform` _returnvalue (`|GetArrayItem` _spawnrotations (`KismetMathLibrary.RandomIntegerInRange` 0 (- (`KismetArrayLibrary.Array_Length` _spawnrotations) 1))) (`/Game/Actors/WorldTiles/BP_WorldTile.WorldScale` (`local.LocalWorldTile`))) "Undefined" "OverrideRootScale" null null))
          (`KismetArrayLibrary.Array_Add` (`self.WorldTileArray`) _returnvalue_3))))))

(fn `SpawnTilePath`
  (params (InEnteredTile :type "/Game/Actors/WorldTiles/BP_WorldTile Object Reference"))
  (locals (SpawnRotation :type "Rotator Structure") (SpawnLocation :type "Vector Structure") (NewLocalVar_0 :type "/Game/Actors/WorldTiles/BP_WorldTile Class Reference") (NewLocalVar_1 :type "Vector Structure" :default (0.0 0.0 0.0)))
  (bind _worldtiletypearray (`self.WorldTileTypeArray`))
  (set `self.EnteredTile` InEnteredTile)
  (`/Engine/EditorBlueprintResources/StandardMacros.IsValid` (`self.LeadingTile`)
    (:`Is Valid`
      _)
    (:`Is Not Valid`
      (set `self.LeadingTile` (`self.EnteredTile`))))
  (for _index (range 1 (+ (`self.TilePathLength`) 1))
    (bind _returnvalue_x (`KismetMathLibrary.BreakVector` (* (* (`BoxComponent.BoxExtent` (`/Game/Actors/WorldTiles/BP_WorldTile.TileBoundaryBox` InEnteredTile)) 2) _index)))
    (bind (_outactors _returnvalue) (`KismetSystemLibrary.CapsuleOverlapActors` (+ (`self.K2_GetActorLocation` (`self.EnteredTile`)) (`KismetMathLibrary.MakeVector` _returnvalue_x)) 1000.0 5000.0 (`|MakeArray` "ObjectTypeQuery7" :!type "EObjectTypeQuery Enum") "/Game/Actors/WorldTiles/BP_WorldTile.BP_WorldTile_C"))
    (if (not _returnvalue)
      (bind _returnvalue_2 (`|SpawnActorFromClass` (`|GetArrayItem` _worldtiletypearray (`KismetMathLibrary.RandomIntegerInRange` 0 (- 0 (`KismetArrayLibrary.Array_Length` _worldtiletypearray)))) (`SceneComponent.K2_GetComponentToWorld` (`/Game/Actors/WorldTiles/BP_WorldTile.Tile1` (`self.LeadingTile`))) "Undefined" "OverrideRootScale" null null))
      (bind _returnvalue_3 (`self.GetCurrentlySpawningTile`))
      (`/Engine/EditorBlueprintResources/StandardMacros.IsValid` _returnvalue_3
        (:`Is Valid`
          _)
        (:`Is Not Valid`
          (`self.SetCurrentlySpawningTile` _returnvalue_2)))
      (bind _asbp_world_tile (cast `/Game/Actors/WorldTiles/BP_WorldTile` _returnvalue_2))
      (`KismetArrayLibrary.Array_Add` (`self.WorldTileArray`) _returnvalue_2)
      (set `self.LeadingTile` _asbp_world_tile))))

(fn `UserConstructionScript`)