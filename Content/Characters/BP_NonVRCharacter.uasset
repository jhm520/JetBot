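; Player character Blueprint for non-VR play, a child class that forwards keyboard and axis input to inherited setters for movement, jumping, grinding, jet, ailerons and braking.
; Look pitch also rotates CameraRoot, clamped just short of straight up or down, while yaw goes only to OnLookYaw.
; Tick defers to the parent and TickLeaning is overridden empty; leftover leaning, friction, ledge and material logic is disconnected and never runs.
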(event `self.ReceiveBeginPlay`)

(event `self.ReceiveTick`
  (params (DeltaSeconds :type "Float (single-precision)"))
  (`parent.ReceiveTick` DeltaSeconds))

(event `self.TickLeaning`
  (params (DeltaTime :type "Float (single-precision)")))

(event `InputAction|MoveForward`
  (params (Key :type "Key Structure"))
  (:`Pressed`
    ;[1 1 1] Leaning, not sure if we'll use this in non vr
    (`self.SetMoveForward` true))
  (:`Released`
    (`self.SetMoveForward` false)))

(event `InputAction|MoveBackward`
  (params (Key :type "Key Structure"))
  (:`Pressed`
    (`self.SetMoveBackward` true))
  (:`Released`
    (`self.SetMoveBackward` false)))

(event `InputAction|Ailerons`
  (params (Key :type "Key Structure"))
  (:`Pressed`
    (`self.SetAilerons` true))
  (:`Released`
    (`self.SetAilerons` false)))

(event `InputAction|MoveLeft`
  (params (Key :type "Key Structure"))
  (:`Pressed`
    (`self.SetMoveLeft` true))
  (:`Released`
    (`self.SetMoveLeft` false)))

(event `InputAction|MoveRight`
  (params (Key :type "Key Structure"))
  (:`Pressed`
    (`self.SetMoveRight` true))
  (:`Released`
    (`self.SetMoveRight` false)))

(event `InputAction|Grind`
  (params (Key :type "Key Structure"))
  (:`Pressed`
    (`self.SetGrind` true))
  (:`Released`
    (`self.SetGrind` false)))

(event `InputAction|Jump`
  (params (Key :type "Key Structure"))
  (:`Pressed`
    (`self.SetJump` true))
  (:`Released`
    (`self.SetJump` false)))

(event `InputAction|Jet`
  (params (Key :type "Key Structure"))
  (:`Pressed`
    (`self.SetJet` true))
  (:`Released`
    (`self.SetJet` false)))

(event `InputAction|Brake`
  (params (Key :type "Key Structure")))

(event `InputAxis|JetAxis`
  (params (AxisValue :type "Float (single-precision)"))
  (`self.SetJetAxis` AxisValue))

(event `InputAxis|MoveForwardAxis`
  (params (AxisValue :type "Float (single-precision)"))
  (`self.SetMoveForwardAxis` AxisValue))

(event `InputAxis|BrakeAxis`
  (params (AxisValue :type "Float (single-precision)"))
  (`self.SetBrakeAxis` AxisValue))

(event `InputAxis|MoveRightAxis`
  (params (AxisValue :type "Float (single-precision)"))
  (`self.SetMoveRightAxis` AxisValue))

(event `InputAxis|LookYaw`
  (params (AxisValue :type "Float (single-precision)"))
  (`self.OnLookYaw` AxisValue))

(event `InputAxis|LookPitch`
  (params (AxisValue :type "Float (single-precision)"))
  (bind (_relativerotation_roll _relativerotation_pitch _relativerotation_yaw) (`KismetMathLibrary.BreakRotator` (`SceneComponent.RelativeRotation` (`self.CameraRoot`))))
  (`self.OnLookPitch` AxisValue)
  (if (< (`KismetMathLibrary.Abs` (+ _relativerotation_pitch AxisValue)) 90.0)
    (`SceneComponent.K2_AddRelativeRotation` (`self.CameraRoot`) (`KismetMathLibrary.MakeRotator` 0.0 AxisValue) false false)
    (else
      (`SceneComponent.K2_SetRelativeRotation` (`self.CameraRoot`) (`KismetMathLibrary.MakeRotator` _relativerotation_roll (* 89.9 (`KismetMathLibrary.SignOfFloat` _relativerotation_pitch)) _relativerotation_yaw) false false))))

(fn `UserConstructionScript`
  (`parent.UserConstructionScript`))