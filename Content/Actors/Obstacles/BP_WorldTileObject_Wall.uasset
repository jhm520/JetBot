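; Wall obstacle for world tiles that gives itself a random orientation and length when spawned by a tile.
; On that spawn event it picks stepped random pitch and yaw, then places copies of its own class along its local Y axis, spaced by the BoundaryBox width.
; An overlap test against other JetBotObstacle actors skips blocked slots, and each new segment is owned by and attached to the previous one.
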(event `/Game/Actors/Obstacles/WorldTileObjectInterface.OnSpawnedByTile`
  (`self.K2_SetActorRotation` (`KismetMathLibrary.MakeRotator` 0.0 (* (`KismetMathLibrary.RandomIntegerInRange` 0 2) 30.0) (* (`KismetMathLibrary.RandomIntegerInRange` 0 7) 45.0)))
  (`self.ExtendWallToRandomLength`))

(fn `ExtendWallToRandomLength`
  (locals (LocalCurrentOwner :type "/Game/Actors/Obstacles/BP_WorldTileObject Object Reference"))
  (bind _localcurrentowner (`local.LocalCurrentOwner`))
  (bind _localcurrentowner_2 (`local.LocalCurrentOwner`))
  (bind _boundarybox (`self.BoundaryBox`))
  (bind _array (`|MakeArray` _localcurrentowner null :!type "Actor Object Reference"))
  (bind (_boxextent_x _boxextent_y) (`KismetMathLibrary.BreakVector` (`BoxComponent.BoxExtent` _boundarybox)))
  (bind _returnvalue (`KismetMathLibrary.RandomIntegerInRange` (- (`self.MinWallLength`) 1) (`self.MaxWallLength`)))
  (if (`KismetMathLibrary.Conv_IntToBool` _returnvalue)
    (set `local.LocalCurrentOwner` self)
    (for _index (range 1 (+ _returnvalue 1))
      (`/Engine/EditorBlueprintResources/StandardMacros.IsValid` _localcurrentowner
        (:`Is Valid`
          (`KismetArrayLibrary.Array_Append` _array (`self.GetAttachedActors`))
          (bind _returnvalue_2 (`KismetMathLibrary.ComposeTransforms` (`KismetMathLibrary.MakeTransform` (`KismetMathLibrary.MakeVector` 0.0 (* _index (* _boxextent_y 2.0)))) (`self.GetTransform`)))
          (bind (_outactors _returnvalue_3) (`KismetSystemLibrary.ComponentOverlapActors` _boundarybox _returnvalue_2 (`|MakeArray` "ObjectTypeQuery9" :!type "EObjectTypeQuery Enum") "/Script/JetBot.JetBotObstacle" _array))
          (if (not _returnvalue_3)
            (bind _returnvalue_4 (`|SpawnActorFromClass` (`GameplayStatics.GetObjectClass` self) _returnvalue_2 "Undefined" "OverrideRootScale" _localcurrentowner_2 null :!label _label))
            (`self.K2_AttachToActor` _returnvalue_4 _localcurrentowner_2 "None" "KeepWorld" "KeepWorld" "KeepWorld" true)
            (set `local.LocalCurrentOwner` _returnvalue_4)))
        (:`Is Not Valid`
          (goto _label))))))

(fn `UserConstructionScript`
  (`parent.UserConstructionScript`))