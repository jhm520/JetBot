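; BP_HideNSeekCharacter is a networked player character with axis-driven movement and look, halving walk speed when moving backwards.
; Movement input follows the capsule's rotation; yaw turns the controller and stores a turn value, printing it for debug.
; Turn yaw, clamped camera pitch and backward state each use an authority switch, forwarding remote calls to server events that re-enter the same setter, so changes apply only on authority.
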(event `self.ReceiveTick`
  (params (DeltaSeconds :type "Float (single-precision)")))

(event `InputAxis|MoveForwardAxis`
  (params (AxisValue :type "Float (single-precision)"))
  (`self.AddMovementInput` (`KismetMathLibrary.GreaterGreater_VectorRotator` (* (1.0 0.0 0.0) AxisValue) (`SceneComponent.K2_GetComponentRotation` (`self.CapsuleComponent`))))
  (`self.SetIsMovingBackwards` (< AxisValue 0.0)))

(event `InputAxis|MoveRightAxis`
  (params (AxisValue :type "Float (single-precision)"))
  (`self.AddMovementInput` (`KismetMathLibrary.GreaterGreater_VectorRotator` (* (0.0 1.0 0.0) AxisValue) (`SceneComponent.K2_GetComponentRotation` (`self.CapsuleComponent`)))))

(event `SetTurnDirection`
  (params (YawAxis :type "Float (double-precision)"))
  ;[1 1 1] SetTurnDirection
  (`/Engine/EditorBlueprintResources/ActorMacros.Switch Has Authority`
    (:`Authority`
      (set `self.TurnYaw` YawAxis))
    (:`Remote`
      (`self.ServerSetTurnDirection` YawAxis))))

(event `InputAxis|LookYaw`
  (params (AxisValue :type "Float (single-precision)"))
  (`|ExecutionSequence`
    (:`then_0`
      (`self.AddControllerYawInput` AxisValue))
    (:`then_1`
      (`KismetSystemLibrary.PrintString` (`KismetStringLibrary.Conv_DoubleToString` AxisValue))
      (`self.SetTurnDirection` AxisValue))))

(event `ServerSetTurnDirection`
  (params (YawAxis :type "Float (double-precision)"))
  ;[1 1 1] SetTurnDirection
  (`self.SetTurnDirection` YawAxis))

(event `InputAxis|LookPitch`
  (params (AxisValue :type "Float (single-precision)"))
  (`self.AddCameraPitch` AxisValue))

(event `ServerAddCameraPitch`
  (params (InPitch :type "Float (double-precision)"))
  (`self.AddCameraPitch` InPitch))

(event `SetIsMovingBackwards`
  (params (bIsMovingBackwards :type Boolean))
  ;[1 1 1] IsMovingBackwards
  (if (!= bIsMovingBackwards (`self.bIsMovingBackwards`))
    (`/Engine/EditorBlueprintResources/ActorMacros.Switch Has Authority`
      (:`Authority`
        (bind _output_get (set `self.bIsMovingBackwards` bIsMovingBackwards))
        (set `CharacterMovementComponent.MaxWalkSpeed` (select `bool` _output_get :`false` 500.0 :`true` 250.0 :!type "Float (single-precision)") (`self.CharacterMovement`)))
      (:`Remote`
        (`self.ServerSetIsMovingBackwards` bIsMovingBackwards)))))

(event `AddCameraPitch`
  (params (InPitch :type "Float (double-precision)"))
  (bind (_relativerotation_roll _relativerotation_pitch) (`KismetMathLibrary.BreakRotator` (`SceneComponent.RelativeRotation` (`self.Camera`))))
  (`/Engine/EditorBlueprintResources/ActorMacros.Switch Has Authority`
    (:`Authority`
      (`SceneComponent.K2_SetRelativeRotation` (`self.Camera`) (`KismetMathLibrary.MakeRotator` 0.0 (`KismetMathLibrary.FClamp` (+ InPitch _relativerotation_pitch) -89.0 89.0)) false false))
    (:`Remote`
      (`self.ServerAddCameraPitch` InPitch))))

(event `ServerSetIsMovingBackwards`
  (params (bIsMovingBackwards :type Boolean))
  ;[1 1 1] IsMovingBackwards
  (`self.SetIsMovingBackwards` bIsMovingBackwards))

(fn `UserConstructionScript`)