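; Column obstacle that serves as a world tile object and varies its orientation when a tile spawns it.
; On the spawned-by-tile event it sets a random rotation in 45-degree steps, with roll and pitch either flat or tilted one step and yaw covering the full circle.
; BeginPlay and the construction script only call the parent.
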(event `/Game/Actors/Obstacles/WorldTileObjectInterface.OnSpawnedByTile`
  (`self.K2_SetActorRotation` (`KismetMathLibrary.MakeRotator` (* (`KismetMathLibrary.RandomIntegerInRange` 0 1) 45.0) (* (`KismetMathLibrary.RandomIntegerInRange` 0 1) 45.0) (* (`KismetMathLibrary.RandomIntegerInRange` 0 7) 45.0))))

(event `self.ReceiveBeginPlay`
  (`parent.ReceiveBeginPlay`))

(fn `UserConstructionScript`
  (`parent.UserConstructionScript`))