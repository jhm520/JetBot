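; VR player character that turns motion controllers and head movement into jetting, jumping and lean steering.
; Spawns left and right JetBot motion controllers, whose pulled triggers enable the jet and sum into a flattened move direction before the parent tick.
; Dropping the head below its calibrated resting height sets jump.
; TickLeaning converts sideways head lean into a velocity-scaled strafe impulse, and an empty TickInputVector overrides that event.
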(event `InputAxis|TriggerLeft`
  (params (AxisValue :type "Float (single-precision)"))
  (set `/Game/Characters/BP_JetBotMotionController.TriggerAxis` AxisValue (`self.LeftHand`)))

(event `InputAxis|TriggerRight`
  (params (AxisValue :type "Float (single-precision)"))
  (set `/Game/Characters/BP_JetBotMotionController.TriggerAxis` AxisValue (`self.RightHand`)))

(event `self.ReceiveBeginPlay`
  (`|ExecutionSequence`
    (:`then_0`
      (bind _returnvalue (`|SpawnActorFromClass` "/Game/Characters/BP_JetBotMotionController.BP_JetBotMotionController_C" (`SceneComponent.K2_GetComponentToWorld` (`self.CameraRoot`)) "Undefined" "OverrideRootScale" self self))
      (`/Game/Characters/BP_JetBotMotionController.SetHand` _returnvalue "Left")
      (bind _output_get (set `self.LeftHand` _returnvalue))
      (`self.K2_AttachToComponent` _output_get (`self.CameraRoot`) "None" "SnapToTarget" "SnapToTarget" "KeepWorld" true))
    (:`then_1`
      (bind _returnvalue_2 (`|SpawnActorFromClass` "/Game/Characters/BP_JetBotMotionController.BP_JetBotMotionController_C" (`SceneComponent.K2_GetComponentToWorld` (`self.CameraRoot`)) "Undefined" "OverrideRootScale" self self))
      (`/Game/Characters/BP_JetBotMotionController.SetHand` _returnvalue_2 "Right")
      (bind _output_get_2 (set `self.RightHand` _returnvalue_2))
      (`self.K2_AttachToComponent` _output_get_2 (`self.CameraRoot`) "None" "SnapToTarget" "SnapToTarget" "KeepWorld" true))))

(event `InputAction|CalibrateHMD`
  (params (Key :type "Key Structure"))
  (bind (_relativelocation_x _relativelocation_y) (`KismetMathLibrary.BreakVector` (`SceneComponent.RelativeLocation` (`self.Camera`))))
  (:`Pressed`
    (`SceneComponent.K2_SetRelativeLocation` (`self.MovementRoot`) (`KismetMathLibrary.MakeVector` _relativelocation_x _relativelocation_y -100.0) false false)
    (set `self.HeadRestingLocation` (`SceneComponent.RelativeLocation` (`self.Camera`)))))

(event `self.ReceiveTick`
  (params (DeltaSeconds :type "Float (single-precision)"))
  (bind (_returnvalue_x _returnvalue_y _returnvalue_z) (`KismetMathLibrary.BreakVector` (- (`SceneComponent.RelativeLocation` (`self.Camera`)) (`self.HeadRestingLocation`))))
  (`|ExecutionSequence`
    (:`then_0`
      (set `self.MoveDirection` (0.0 0.0 0.0))
      (`self.SetJet` false)
      (if (or (>= (`/Game/Characters/BP_JetBotMotionController.TriggerAxis` (`self.LeftHand`)) 0.9) (>= (`/Game/Characters/BP_JetBotMotionController.TriggerAxis` (`self.RightHand`)) 0.9))
        (`self.SetJet` true)
        (`|ExecutionSequence`
          (:`then_0`
            (if (>= (`/Game/Characters/BP_JetBotMotionController.TriggerAxis` (`self.LeftHand`)) 0.9)
              (set `self.MoveDirection` (`/Game/Characters/BP_JetBotMotionController.GetMoveDirection` (`self.LeftHand`)))))
          (:`then_1`
            (if (>= (`/Game/Characters/BP_JetBotMotionController.TriggerAxis` (`self.RightHand`)) 0.9)
              (set `self.MoveDirection` (+ (`self.MoveDirection`) (`/Game/Characters/BP_JetBotMotionController.GetMoveDirection` (`self.RightHand`)))))))
        (else
          (set `self.MoveDirection` (0.0 0.0 0.0)))))
    (:`then_1`
      (if (< _returnvalue_z -20.0)
        (`self.SetJump` true)
        (else
          (`self.SetJump` false))))
    (:`then_2`
      (set `self.MoveDirection` (* (`self.MoveDirection`) (1.0 1.0 0.0)))
      (bind _output_get (set `self.MoveDirection` (`KismetMathLibrary.Normal` (`self.MoveDirection`))))
      (`parent.ReceiveTick` DeltaSeconds))))

(event `TickInputVector`)

(event `self.TickLeaning`
  (params (DeltaTime :type "Float (single-precision)"))
  (set `self.LeanAngle` (`KismetMathLibrary.DegAtan` (/ (.y (`KismetMathLibrary.InverseTransformLocation` (`SceneComponent.K2_GetComponentToWorld` (`self.MovementDirection`)) (`SceneComponent.K2_GetComponentLocation` (`self.Camera`)))) (.z (`KismetMathLibrary.InverseTransformLocation` (`SceneComponent.K2_GetComponentToWorld` (`self.MovementDirection`)) (`SceneComponent.K2_GetComponentLocation` (`self.Camera`)))))))
  (`CharacterMovementComponent.AddImpulse` (`self.CharacterMovement`) (* (* (`SceneComponent.GetRightVector` (`self.MovementDirection`)) (* (* (`self.LeanAngle`) DeltaTime) (* (`KismetMathLibrary.VSize` (`MovementComponent.Velocity` (`self.CharacterMovement`))) 4.0))) DeltaTime) true))

(fn `UserConstructionScript`
  (`parent.UserConstructionScript`))