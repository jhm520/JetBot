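; BP_Monster is a monster character Blueprint whose point light is meant to be seen only by the player controlling it.
; On BeginPlay it hides the PointLight on any instance that is not locally controlled, then calls the parent's BeginPlay.
; The construction script only calls the parent, and the Tick and overlap events are disabled stubs.
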(event `self.ReceiveBeginPlay`
  (`|ExecutionSequence`
    (:`then_0`
      (if (not (`self.IsLocallyControlled`))
        (`SceneComponent.SetVisibility` (`self.PointLight`) false false)))
    (:`then_1`
      (`parent.ReceiveBeginPlay`))))

(fn `UserConstructionScript`
  (`parent.UserConstructionScript`))