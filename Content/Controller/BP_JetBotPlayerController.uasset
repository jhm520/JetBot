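; Player controller for the JetBot game that respawns the player's character whenever it is destroyed.
; On BeginPlay it binds to the possessed pawn's OnDestroyed event, if that pawn is valid.
; When that event fires, it spawns a BP_JetBotCharacter at the first PlayerStart found, possesses it and binds the same handler, so respawning repeats.
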(event `self.ReceiveBeginPlay`
  (bind _returnvalue (`self.K2_GetPawn`))
  (`/Engine/EditorBlueprintResources/StandardMacros.IsValid` _returnvalue
    (:`Is Valid`
      (add `self.OnDestroyed` _returnvalue (delegate `OnDestroyed_Event_0`)))))

(event `OnDestroyed_Event_0` :!signature `self.OnDestroyed`
  (params (DestroyedActor :type "Actor Object Reference"))
  (bind _outactors (`GameplayStatics.GetAllActorsOfClass` "/Script/Engine.PlayerStart"))
  (bind _output (`|GetArrayItem` _outactors))
  (`/Engine/EditorBlueprintResources/StandardMacros.IsValid` _output
    (:`Is Valid`
      (bind _returnvalue (`|SpawnActorFromClass` "/Game/Characters/BP_JetBotCharacter.BP_JetBotCharacter_C" (`self.GetTransform` _output) "Undefined" "OverrideRootScale"))
      (`self.Possess` _returnvalue)
      (add `self.OnDestroyed` _returnvalue (delegate `OnDestroyed_Event_0`)))))

(fn `UserConstructionScript`)