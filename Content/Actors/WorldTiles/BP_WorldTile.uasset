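; World tile actor for the JetBot level that scatters random obstacles through its volume.
; On BeginPlay it destroys itself if overlapping the player or over BP_LevelSpawner's tile cap, otherwise registers there and spawns game-mode object types at random points in TileObstacleBox.
; SpawnSurroundingTiles recursively adds randomly rotated, height-offset neighbors where a capsule trace is clear.
; Grid-based spawning and tile-enter detection are disconnected from the event graph.
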(event `SpawnObstacles`
  (bind _tileobstaclebox (`self.TileObstacleBox`))
  (for _ (range (+ (`self.NumObjects`) 1))
    (bind _asbp_jet_bot_game_mode (cast `/Game/GameMode/BP_JetBotGameMode` (`GameplayStatics.GetGameMode`)))
    (bind _tileobjecttypes (`/Game/GameMode/BP_JetBotGameMode.TileObjectTypes` _asbp_jet_bot_game_mode))
    (`|SpawnActorFromClass` (`|GetArrayItem` _tileobjecttypes (`KismetMathLibrary.RandomIntegerInRange` 0 (- (`KismetArrayLibrary.Array_Length` _tileobjecttypes) 1))) (`KismetMathLibrary.MakeTransform` (+ (`SceneComponent.K2_GetComponentLocation` _tileobstaclebox) (* (`BoxComponent.GetScaledBoxExtent` _tileobstaclebox) (`KismetMathLibrary.MakeVector` (`KismetMathLibrary.RandomFloatInRange` -1.0 1.0) (`KismetMathLibrary.RandomFloatInRange` -1.0 1.0) (`KismetMathLibrary.RandomFloatInRange` -1.0 1.0))))) "AlwaysSpawn" "OverrideRootScale" self null)))

(event `self.ReceiveBeginPlay`
  (`|ExecutionSequence`
    (:`then_0`
      (bind _asbp_level_spawner (cast `/Game/Actors/BP_LevelSpawner` (`self.GetOwner`)))
      (if (`self.IsOverlappingActor` (`GameplayStatics.GetPlayerPawn` 0))
        (`self.K2_DestroyActor` :!label _label)
        (else
          (bind _tilearray (`/Game/Actors/BP_LevelSpawner.TileArray` _asbp_level_spawner))
          (if (>= (`KismetArrayLibrary.Array_Length` _tilearray) (`/Game/Actors/BP_LevelSpawner.MaxTiles` _asbp_level_spawner))
            (goto _label)
            (else
              (`KismetArrayLibrary.Array_Add` _tilearray self)
              (`|ExecutionSequence`
                (:`then_0`
                  (`self.SpawnObstacles`))))))))))

(event `DelaySpawningTiles`)

(event `self.TileObstacleBox.OnComponentBeginOverlap`
  (params (OverlappedComponent :type "PrimitiveComponent Object Reference") (OtherActor :type "Actor Object Reference") (OtherComp :type "PrimitiveComponent Object Reference") (OtherBodyIndex :type Integer) (bFromSweep :type Boolean) (SweepResult :type "HitResult Structure (by ref)")))

(event `self.ReceiveTick`
  (params (DeltaSeconds :type "Float (single-precision)")))

(event `SpawnObstacleOnTile_1`)

(fn `CalculateObjectSpawnTransforms`
  (locals (LocalXIndex :type Integer) (LocalYIndex :type Integer) (LocalZIndex :type Integer))
  (bind _returnvalue (`KismetMathLibrary.Conv_IntToDouble` 0))
  (bind _returnvalue_2 (`KismetMathLibrary.Conv_IntToDouble` 0))
  (bind (_returnvalue_x _returnvalue_y) (`KismetMathLibrary.BreakVector` (`BoxComponent.GetUnscaledBoxExtent` (`self.TileObstacleBox`))))
  (bind _returnvalue_x_2 (`KismetMathLibrary.BreakVector` (`BoxComponent.GetUnscaledBoxExtent` (`self.TileObstacleBox`))))
  (`KismetArrayLibrary.Array_Clear` (`self.ObjectSpawnTransforms`))
  (for _index (range (+ (`KismetMathLibrary.FTrunc` (/ (* _returnvalue_x_2 2.0) _returnvalue)) 1))
    (bind _returnvalue_3 (+ _returnvalue_x_2 (* _index (* _returnvalue -1.0))))
    (if (not (>= (`KismetMathLibrary.Abs` _returnvalue_3) _returnvalue_x_2))
      (for _index_2 (range (+ (`KismetMathLibrary.FTrunc` (/ (* _returnvalue_y 2.0) _returnvalue_2)) 1))
        (bind _returnvalue_4 (+ (* _returnvalue_y -1.0) (* _index_2 _returnvalue_2)))
        (if (not (>= (`KismetMathLibrary.Abs` _returnvalue_4) _returnvalue_y))
          (`KismetArrayLibrary.Array_Add` (`self.ObjectSpawnTransforms`) (`KismetMathLibrary.MakeTransform` (`KismetMathLibrary.MakeVector` _returnvalue_3 _returnvalue_4))))))))

(fn `IsPlayerFarAway`
  (returns (bFarAway :type Boolean))
  (bind _boxextent_x (`KismetMathLibrary.BreakVector` (`BoxComponent.BoxExtent` (`self.TileObstacleBox`))))
  (bind _returnvalue (+ (* (/ (`self.TileClusterSquareRoot`) 2) (* _boxextent_x 2.0)) (/ _boxextent_x 2.0)))
  (return (> (`KismetMathLibrary.VSize` (- (`self.K2_GetActorLocation` (`GameplayStatics.GetPlayerCharacter` 0)) (`self.K2_GetActorLocation`))) (`KismetMathLibrary.VSize` (`KismetMathLibrary.MakeVector` _returnvalue _returnvalue _returnvalue)))))

(fn `OnEnterTile`
  (locals (PreviousCenterTile :type "Object Object Reference"))
  (bind _asbp_jet_bot_game_mode (cast `/Game/GameMode/BP_JetBotGameMode` (`GameplayStatics.GetGameMode`)))
  (`/Game/GameMode/BP_JetBotGameMode.OnTileEntered` _asbp_jet_bot_game_mode self))

(fn `OrientTileToWorld`)

(fn `SpawnNextObjectOnTile`
  (set `self.CurrentObjectSpawnTransformIndex` (+ (`self.CurrentObjectSpawnTransformIndex`) (`KismetMathLibrary.RandomIntegerInRange` 0)))
  (if (< (`self.CurrentObjectSpawnTransformIndex`) (`KismetArrayLibrary.Array_Length` (`self.ObjectSpawnTransforms`)))
    (bind _asbp_jet_bot_game_mode (cast `/Game/GameMode/BP_JetBotGameMode` (`GameplayStatics.GetGameMode`)))
    (bind _tileobjecttypes (`/Game/GameMode/BP_JetBotGameMode.TileObjectTypes` _asbp_jet_bot_game_mode))
    (bind _returnvalue (`|SpawnActorFromClass` (`|GetArrayItem` _tileobjecttypes (`KismetMathLibrary.RandomIntegerInRange` 0 (- (`KismetArrayLibrary.Array_Length` _tileobjecttypes) 1))) (`KismetMathLibrary.ConvertTransformToRelative` (`|GetArrayItem` (`self.ObjectSpawnTransforms`) (`self.CurrentObjectSpawnTransformIndex`)) (`self.GetTransform`)) "Undefined" "OverrideRootScale" self null))
    (if (`PrimitiveComponent.IsOverlappingActor` (`/Game/Actors/Obstacles/BP_WorldTileObject.BoundaryBox` _returnvalue) (`GameplayStatics.GetPlayerCharacter` 0))
      (`self.K2_DestroyActor` _returnvalue))
    (else
      (`self.SetActorTickEnabled` false))))

(fn `SpawnObject`
  (params (Spawner :type "PrimitiveComponent Object Reference"))
  (if (`KismetMathLibrary.Conv_IntToBool` (`KismetMathLibrary.RandomIntegerInRange` 0 500))
    _
    (elif (not (`PrimitiveComponent.IsOverlappingActor` Spawner (`GameplayStatics.GetPlayerCharacter` 0)))
      (`/Engine/EditorBlueprintResources/StandardMacros.IsValid` (`|GetArrayItem` (`PrimitiveComponent.GetOverlappingActors` Spawner "/Game/Actors/Obstacles/BP_WorldTileObject.BP_WorldTileObject_C"))
        (:`Is Not Valid`
          (bind _asbp_jet_bot_game_mode (cast `/Game/GameMode/BP_JetBotGameMode` (`GameplayStatics.GetGameMode`)))
          (bind _tileobjecttypes (`/Game/GameMode/BP_JetBotGameMode.TileObjectTypes` _asbp_jet_bot_game_mode))
          (`|SpawnActorFromClass` (`|GetArrayItem` _tileobjecttypes (`KismetMathLibrary.RandomIntegerInRange` 0 (- (`KismetArrayLibrary.Array_Length` _tileobjecttypes) 1))) (`SceneComponent.K2_GetComponentToWorld` Spawner) "Undefined" "OverrideRootScale" self null))))))

(fn `SpawnObjectsOnTile`
  (locals (LocalObjectSpawnTransformIndex :type Integer) (LocalGameMode :type "/Game/GameMode/BP_JetBotGameMode Object Reference") (LocalXPos :type Integer :default -5000) (LocalYPos :type Integer :default -5000) (LocalZPos :type Integer :default 0) (LocalXPosMax :type Integer :default 5000) (LocalYPosMax :type Integer :default 5000) (LocalZPosMax :type Integer :default 10000))
  (bind _returnvalue (`KismetMathLibrary.RandomIntegerInRange` 0))
  (bind _returnvalue_2 (`KismetMathLibrary.RandomIntegerInRange` 0))
  (bind _returnvalue_3 (`KismetMathLibrary.RandomIntegerInRange` 0))
  (bind _returnvalue_4 (`KismetMathLibrary.RandomIntegerInRange` 0))
  (bind _returnvalue_location (`KismetMathLibrary.BreakTransform` (`self.GetTransform`)))
  (bind _returnvalue_5 (`KismetMathLibrary.RandomIntegerInRange` 0))
  (bind _returnvalue_6 (`KismetMathLibrary.RandomIntegerInRange` 0))
  (bind _tileobjecttypes (`/Game/GameMode/BP_JetBotGameMode.TileObjectTypes` (`local.LocalGameMode`)))
  (bind _asbp_jet_bot_game_mode (cast `/Game/GameMode/BP_JetBotGameMode` (`GameplayStatics.GetGameMode`)))
  (set `local.LocalGameMode` _asbp_jet_bot_game_mode)
  (set `local.LocalXPos` (+ (`local.LocalXPos`) (- _returnvalue_5 (mod _returnvalue_5 1))))
  (while (< (`local.LocalXPos`) (`local.LocalXPosMax`))
    (set `local.LocalYPos` (+ (`local.LocalYPos`) (- _returnvalue_4 (mod _returnvalue_4 1))))
    (while (< (`local.LocalYPos`) (`local.LocalYPosMax`))
      (while (< (`local.LocalZPos`) (`local.LocalZPosMax`))
        (bind _returnvalue_7 (`KismetArrayLibrary.Array_Add` (`self.ObjectSpawnTransforms`) (`KismetMathLibrary.MakeTransform` (`KismetMathLibrary.MakeVector` (`KismetMathLibrary.Conv_IntToDouble` (`local.LocalXPos`)) (`KismetMathLibrary.Conv_IntToDouble` (`local.LocalYPos`)) (`KismetMathLibrary.Conv_IntToDouble` (`local.LocalZPos`))))))
        (set `local.LocalZPos` (+ (`local.LocalZPos`) (- _returnvalue_2 (mod _returnvalue_2 1))))
        (bind _returnvalue_8 (`|SpawnActorFromClass` (`|GetArrayItem` _tileobjecttypes (`KismetMathLibrary.RandomIntegerInRange` 0 (- (`KismetArrayLibrary.Array_Length` _tileobjecttypes) 1))) (`KismetMathLibrary.MakeTransform` (+ (.location (`|GetArrayItem` (`self.ObjectSpawnTransforms`) _returnvalue_7)) _returnvalue_location)) "Undefined" "OverrideRootScale" self null))
        (if (`PrimitiveComponent.IsOverlappingActor` (`/Game/Actors/Obstacles/BP_WorldTileObject.BoundaryBox` _returnvalue_8) (`GameplayStatics.GetPlayerCharacter` 0))
          (`self.K2_DestroyActor` _returnvalue_8)))
      (set `local.LocalZPos` 0)
      (set `local.LocalYPos` (+ (`local.LocalYPos`) (- _returnvalue_3 (mod _returnvalue_3 1)))))
    (set `local.LocalXPos` (+ (`local.LocalXPos`) (- _returnvalue (mod _returnvalue 1))))
    (set `local.LocalYPos` -5000))
  (set `local.LocalZPos` (+ (`local.LocalZPos`) (- _returnvalue_6 (mod _returnvalue_6 1))))
  (set `local.LocalXPos` -5000))

(fn `SpawnSurroundingTiles`
  (locals (SpawnedTiles :type "Array of /Game/Actors/WorldTiles/BP_WorldTile Object Reference"))
  (bind _returnvalue (`self.GetOwner`))
  (for _array_element (`self.SurroundingTiles`)
    (bind _asbp_level_spawner (cast `/Game/Actors/BP_LevelSpawner` _returnvalue))
    (bind _returnvalue_2 (`KismetMathLibrary.MakeVector` (.x (`SceneComponent.K2_GetComponentLocation` _array_element)) (.y (`SceneComponent.K2_GetComponentLocation` _array_element)) (+ (.z (`SceneComponent.K2_GetComponentLocation` _array_element)) (* (`KismetMathLibrary.RandomIntegerInRange` -1 1) (.z (`BoxComponent.GetScaledBoxExtent` (`self.TileBoundaryBox`)))))))
    (bind (_outhit _returnvalue_3) (`KismetSystemLibrary.CapsuleTraceSingleForObjects` _returnvalue_2 (- _returnvalue_2 (0.0 0.0 3000.0)) 500.0 3000.0 (`|MakeArray` "ObjectTypeQuery7" "ObjectTypeQuery3" :!type "EObjectTypeQuery Enum")))
    (if _returnvalue_3
      (`KismetSystemLibrary.PrintString` "Did not spawn tile")
      (else
        (cast `/Game/Actors/BP_LevelSpawner` (`self.GetOwner`))
        (bind _tileclasses (`/Game/Actors/BP_LevelSpawner.TileClasses` _asbp_level_spawner))
        (bind _returnvalue_4 (`|SpawnActorFromClass` (`|GetArrayItem` _tileclasses (`KismetMathLibrary.RandomIntegerInRange` 0 (- (`KismetArrayLibrary.Array_Length` _tileclasses) 1))) (`KismetMathLibrary.MakeTransform` _returnvalue_2 (`KismetMathLibrary.MakeRotator` 0.0 0.0 (* (`KismetMathLibrary.RandomIntegerInRange` 0 3) 90.0))) "Undefined" "OverrideRootScale" _returnvalue null))
        (`/Engine/EditorBlueprintResources/StandardMacros.IsValid` _returnvalue_4
          (:`Is Valid`
            (`KismetArrayLibrary.Array_Add` (`local.SpawnedTiles`) _returnvalue_4))))))
  (for _array_element_2 (`local.SpawnedTiles`)
    (`/Engine/EditorBlueprintResources/StandardMacros.IsValid` _array_element_2
      (:`Is Valid`
        (`self.SpawnSurroundingTiles` _array_element_2)))))

(fn `UserConstructionScript`
  (locals (ConnectedTileLocation :type "Vector Structure") (TileX :type "Float (double-precision)") (TileY :type "Float (double-precision)"))
  (set `self.SurroundingTiles` (`|MakeArray` (`self.Tile0`) (`self.Tile1`) (`self.Tile2`) (`self.Tile3`) (`self.Tile5`) (`self.Tile6`) (`self.Tile7`) (`self.Tile8`)))
  (set `self.TileCorners` (`|MakeArray` (`self.Corner0`) (`self.Corner1`) (`self.Corner2`) (`self.Corner3`))))